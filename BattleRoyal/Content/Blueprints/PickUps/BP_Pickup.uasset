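; BP_Pickup is a pickup actor with a spinning mesh and sphere-based character detection, providing empty enter and leave events.
; Tick spins PickupMesh around yaw and resets its world roll and pitch to keep it upright.
; PickupSphere overlaps cast to BRCharacter before calling PickupSphereEntered or PickupSphereLeft, which have no logic here.
; The sphere's hit event turns off its physics simulation.
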(event OnComponentHit(PickupSphere)
  (params (HitComponent :type Primitive%20Component%20Object%20Reference) (OtherActor :type Actor%20Object%20Reference) (OtherComp :type Primitive%20Component%20Object%20Reference) (NormalImpulse :type Vector :default "0, 0, 0") (Hit :type Hit%20Result%20Structure%20%28by%20ref%29))
  (Physics|SetSimulatePhysics (Variables|Default|GetPickupSphere) false))

(event OnComponentBeginOverlap(PickupSphere)
  (params (OverlappedComponent :type Primitive%20Component%20Object%20Reference) (OtherActor :type Actor%20Object%20Reference) (OtherComp :type Primitive%20Component%20Object%20Reference) (OtherBodyIndex :type Integer) (bFromSweep :type Boolean) (SweepResult :type Hit%20Result%20Structure%20%28by%20ref%29))
  (bind _asbrcharacter (Utilities|Casting|CastToBRCharacter OtherActor))
  (CallFunction|PickupSphereEntered _asbrcharacter))

(event OnComponentEndOverlap(PickupSphere)
  (params (OverlappedComponent :type Primitive%20Component%20Object%20Reference) (OtherActor :type Actor%20Object%20Reference) (OtherComp :type Primitive%20Component%20Object%20Reference) (OtherBodyIndex :type Integer))
  (bind _asbrcharacter (Utilities|Casting|CastToBRCharacter OtherActor))
  (CallFunction|PickupSphereLeft _asbrcharacter))

(event Custom|PickupSphere%20Entered
  (params (Character :type BR%20Character%20Object%20Reference)))

(event Custom|Pickup%20Sphere%20Left
  (params (Character :type BR%20Character%20Object%20Reference)))

(event EventTick
  (params (DeltaSeconds :type Float%20%28single-precision%29))
  (bind _pickupmesh (Variables|Default|GetPickupMesh))
  ;[1 1 1] Make Pickup Mesh spin and dispose of roll/pitch component
  (Transformation|AddRelativeRotation _pickupmesh (Math|Rotator|MakeRotator 0.0 0.0 (* DeltaSeconds 1.8e+02)) false false)
  (Transformation|SetWorldRotation (Variables|Default|GetPickupMesh) (Math|Rotator|MakeRotator 0.0 0.0 (.Yaw (Math|Rotator|BreakRotator (Transformation|GetWorldRotation _pickupmesh)))) false false))

(fn ConstructionScript)