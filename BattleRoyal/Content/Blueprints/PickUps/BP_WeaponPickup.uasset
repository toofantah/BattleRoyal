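; BP_WeaponPickup is a weapon pickup that holds a weapon class to give along with its clip and spare ammo counts.
; On BeginPlay the server fills both counts from that class's defaults, unless a player dropped the weapon, so dropped weapons keep their remaining ammo.
; Pickup sphere events register it as the character's current weapon pickup on entry and clear it on exit only if it is still current.
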(event EventPickupSphereEntered
  (params (Character :type BR%20Character%20Object%20Reference))
  ;[1 1 1] Set Player Pickup
  (Variables|/Game/FirstPersonBP/Blueprints/BRCharacter.BRCharacter_C|SetCurrentWeaponPickup Character self))

(event EventPickupSphereLeft
  (params (Character :type BR%20Character%20Object%20Reference))
  ;[1 1 1] Unset Player Pickup
  (if (== (Variables|/Game/FirstPersonBP/Blueprints/BRCharacter.BRCharacter_C|GetCurrentWeaponPickup Character) self)
    (Variables|/Game/FirstPersonBP/Blueprints/BRCharacter.BRCharacter_C|SetCurrentWeaponPickup Character 0)))

(event EventBeginPlay
  (bind _weapontogive (Variables|Default|GetWeaponToGive))
  (bind (_damage _weaponname _currentammo _currentspareammo) (Utilities|GetClassDefaults _weapontogive))
  ;[1 1 1] Remember ammo amounts if player dropped weapon
  (Networking|SwitchHasAuthority
    (:Authority
      (if (not (Variables|Default|GetDroppedByPlayer))
        (Variables|Default|SetCurrentAmmoInClip _currentammo)
        (Variables|Default|SetCurrentSpareAmmo _currentspareammo)))))

(fn ConstructionScript
  (|CallParentFunction))