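; BP_Weapon is a weapon Blueprint that manages clip and spare ammo for its owning BRCharacter.
; On the server, BeginPlay initializes ammo and caches the owner, while OnFired spends a round and triggers Reload when the clip empties.
; Reload flags the owner as reloading, then refills the clip from spare ammo after a fixed delay.
; GiveAmmo, also authority-only, tops up the clip before capped spare ammo, and HasAmmo reports whether rounds remain loaded.
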(event Custom|Give%20Ammo
  (params (Ammo%20to%20Give :type Integer))
  ;[1 1 1] An event to give ammo to the weapon when needed
  (Networking|SwitchHasAuthority
    (:Authority
      (Variables|Ammo|SetCurrentAmmo (+ (Variables|Ammo|GetCurrentAmmo) (Math|Integer|Min(Integer) Ammo%20to%20Give (- (Variables|Ammo|GetClipSize) (Variables|Ammo|GetCurrentAmmo)))))
      (if (> (- Ammo%20to%20Give (Math|Integer|Min(Integer) Ammo%20to%20Give (- (Variables|Ammo|GetClipSize) (Variables|Ammo|GetCurrentAmmo)))) 0)
        (Variables|Ammo|SetCurrentSpareAmmo (+ (Variables|Ammo|GetCurrentSpareAmmo) (Math|Integer|Min(Integer) (- Ammo%20to%20Give (Math|Integer|Min(Integer) Ammo%20to%20Give (- (Variables|Ammo|GetClipSize) (Variables|Ammo|GetCurrentAmmo)))) (- (Variables|Ammo|GetMaxSpareAmmo) (Variables|Ammo|GetCurrentSpareAmmo)))))))))

(event Custom|On%20Fired
  (bind _currentammo (Variables|Ammo|GetCurrentAmmo))
  ;[1 1 1] When we fire gun take ammo from player && Reload if needed
  (Networking|SwitchHasAuthority
    (:Authority
      (Math|Integer|DecrementInt _currentammo
        (:%20%20
          (if (<= _currentammo 0)
            (CallFunction|Reload)))))))

(event Custom|Reload
  ;[1 1 1] Reload the Weapon && play Animation
  (Variables|/Game/FirstPersonBP/Blueprints/BRCharacter.BRCharacter_C|SetIsReloading (Variables|Default|GetCurrentOwner) true)
  (Utilities|FlowControl|Delay 2.0)
  (Variables|Ammo|SetCurrentAmmo (Math|Integer|Min(Integer) (Variables|Ammo|GetCurrentSpareAmmo) (Variables|Ammo|GetClipSize)))
  (Variables|Ammo|SetCurrentSpareAmmo (Math|Integer|Max(Integer) (- (Variables|Ammo|GetCurrentSpareAmmo) (Math|Integer|Min(Integer) (Variables|Ammo|GetCurrentSpareAmmo) (Variables|Ammo|GetClipSize)))))
  (Variables|/Game/FirstPersonBP/Blueprints/BRCharacter.BRCharacter_C|SetIsReloading (Variables|Default|GetCurrentOwner) false))

(event EventBeginPlay
  ;[1 1 1] On beginplay ; Setup our ammo amounts
  (Networking|SwitchHasAuthority
    (:Authority
      (Variables|Ammo|SetCurrentAmmo (Variables|Ammo|GetClipSize))
      (Variables|Ammo|SetCurrentSpareAmmo (Variables|Ammo|GetStartingSpareAmmo))
      (bind _asbrcharacter (Utilities|Casting|CastToBRCharacter (Components|GetOwner)))
      (Variables|Default|SetCurrentOwner _asbrcharacter))))

(fn ConstructionScript)

(fn HasAmmo
  (return (> (Variables|Ammo|GetCurrentAmmo) 0)))